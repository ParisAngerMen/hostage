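; BP_Door is a door that watches the player's kill progress to decide when it counts as open.
; On BeginPlay it caches the BP_Player_Controller and starts a looping timer that polls its EnemiesDown count instead of using Tick.
; Once that count reaches EnemiesToOpen, it prints "OPEN" and clears the timer, with no door movement or collision change implemented.
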(event Custom|CheckDoor
  (if (>= (Variables|/Game/InfimaGames/FreeFPSTemplate/Core/BP_Player_Controller.BP_Player_Controller_C|GetenemiesDown (Variables|Default|GetAs%20BP%20Player%20Controller)) (Variables|Default|GetEnemiesToOpen))
    (Development|PrintText "OPEN")
    (Utilities|Time|ClearandInvalidateTimerbyHandle (stale EventBeginPlay _returnvalue))))

(event EventBeginPlay
  (bind _asbp_player_controller (Utilities|Casting|CastToBP_Player_Controller (Game|GetPlayerController 0)))
  (Variables|Default|SetAs%20BP%20Player%20Controller _asbp_player_controller)
  (bind _returnvalue (Utilities|Time|SetTimerbyEvent (delegate Custom|CheckDoor) 1.0 true)))

(event Collision|EventActorBeginOverlap
  (params (OtherActor :type Actor%20Object%20Reference)))

(event EventTick
  (params (DeltaSeconds :type Float%20%28single-precision%29)))

(fn ConstructionScript)