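; BP_AIMovement moves its actor around a looping route of placed patrol point actors, starting at BeginPlay.
; A latent MoveComponentTo slides the root component to the current point over TimeToPatrol, keeping the actor's rotation.
; PatrolIndex then increments, wraps to zero past the last point, and feeds the next move in an endless loop, with no navigation or pathfinding.
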(event EventBeginPlay
  (|CallParentFunction)
  (Components|MoveComponentTo (Variables|Transformation|GetRootComponent) (Transformation|GetActorLocation (Utilities|Array|Get(acopy) (Variables|Default|GetpatrolPoints) (Variables|Default|GetpatrolIndex))) (Transformation|GetActorRotation) false false (Variables|Default|GettimeToPatrol) false :!label _label)
  (Math|Integer|IncrementInt (Variables|Default|GetpatrolIndex)
    (:%20%20
      (if (>= (Variables|Default|GetpatrolIndex) (Utilities|Array|Length (Variables|Default|GetpatrolPoints)))
        (Variables|Default|SetpatrolIndex 0)
        (goto _label)
        (else
          (goto _label))))))

(fn ConstructionScript
  (|CallParentFunction))