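; BP_AI is an enemy in the FPS template that ragdolls when it takes any damage and rewards the player.
; On BeginPlay it caches the player's BP_Player_Controller.
; Any damage enables physics simulation on the skeletal mesh; the first hit also adds bonus time to the controller's countdown, increments its enemies-down count and sets IsDead to prevent repeat rewards.
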(event EventBeginPlay
  (bind _asbp_player_controller (Utilities|Casting|CastToBP_Player_Controller (Game|GetPlayerController 0)))
  (Variables|Default|SetAs%20BP%20Player%20Controller _asbp_player_controller))

(event Game|Damage|EventAnyDamage
  (params (Damage :type Float%20%28single-precision%29) (DamageType :type Damage%20Type%20Object%20Reference) (InstigatedBy :type Controller%20Object%20Reference) (DamageCauser :type Actor%20Object%20Reference))
  ;[1 0.08915 0 1 11] This is where we ragdoll the entire character, it is as simple as this, yep!
  (Physics|SetSimulatePhysics (Variables|Default|GetSkeletalMesh) true)
  (if (not (Variables|Default|GetisDead))
    (Variables|/Game/InfimaGames/FreeFPSTemplate/Core/BP_Player_Controller.BP_Player_Controller_C|SettimeLeft (Variables|Default|GetAs%20BP%20Player%20Controller) (+ (Variables|/Game/InfimaGames/FreeFPSTemplate/Core/BP_Player_Controller.BP_Player_Controller_C|GettimeLeft (Variables|Default|GetAs%20BP%20Player%20Controller)) (Variables|Default|GettimeToAdd)))
    (bind _result (Math|Integer|IncrementInt (Variables|/Game/InfimaGames/FreeFPSTemplate/Core/BP_Player_Controller.BP_Player_Controller_C|GetenemiesDown (Variables|Default|GetAs%20BP%20Player%20Controller)))
      (:%20%20
        (Variables|/Game/InfimaGames/FreeFPSTemplate/Core/BP_Player_Controller.BP_Player_Controller_C|SetenemiesDown (Variables|Default|GetAs%20BP%20Player%20Controller) _result)
        (Variables|Default|SetisDead true)))))

(fn ConstructionScript)